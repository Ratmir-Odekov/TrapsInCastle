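; Trap inventory component that tracks the selected trap slot across floor, wall and ceiling trap lists.
; Mouse wheel up and down trigger events that step an index through three hardcoded slots per list.
; Passing either end wraps into the neighboring list, cycling floor, ceiling, wall upward and the reverse downward.
; Each step prints the new index to screen; no trap data or placement is handled here.
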(event `Key|MouseScrollUp`
  (params (Key :type "Key Structure"))
  (:`Pressed`
    (`self.UpInTrapList`)))

(event `UpInTrapList`
  (bind _returnvalue (+ (`self.TrapInvenoryIndex`) 1))
  (bind _returnvalue_2 (+ (`self.TrapInvenoryIndex`) 1))
  (bind _returnvalue_3 (+ (`self.TrapInvenoryIndex`) 1))
  (switch `/Game/_MyContent/Enums/Enum_TrapInvetoryList` (`self.TrapList`)
    (:`NewEnumerator0`
      (if (== _returnvalue_3 3)
        (set `self.TrapList` "NewEnumerator2")
        (set `self.TrapInvenoryIndex` 0 :!label _label)
        (else
          (set `self.TrapInvenoryIndex` _returnvalue_3))))
    (:`NewEnumerator1`
      (if (== _returnvalue_2 3)
        (set `self.TrapList` "NewEnumerator0")
        (goto _label)
        (else
          (set `self.TrapInvenoryIndex` _returnvalue_2))))
    (:`NewEnumerator2`
      (if (== _returnvalue 3)
        (set `self.TrapList` "NewEnumerator1")
        (goto _label)
        (else
          (set `self.TrapInvenoryIndex` _returnvalue)))))
  (`KismetSystemLibrary.PrintString` (`KismetStringLibrary.Conv_IntToString` (`self.TrapInvenoryIndex`))))

(event `Key|MouseScrollDown`
  (params (Key :type "Key Structure"))
  (:`Pressed`
    (`self.DownInTrapList`)))

(event `DownInTrapList`
  (bind _returnvalue (- (`self.TrapInvenoryIndex`) 1))
  (bind _returnvalue_2 (- (`self.TrapInvenoryIndex`) 1))
  (bind _returnvalue_3 (- (`self.TrapInvenoryIndex`) 1))
  (switch `/Game/_MyContent/Enums/Enum_TrapInvetoryList` (`self.TrapList`)
    (:`NewEnumerator0`
      (if (== _returnvalue_2 -1)
        (set `self.TrapList` "NewEnumerator1")
        (set `self.TrapInvenoryIndex` 2 :!label _label_2)
        (else
          (set `self.TrapInvenoryIndex` _returnvalue_2))))
    (:`NewEnumerator1`
      (if (== _returnvalue_3 -1)
        (set `self.TrapList` "NewEnumerator2")
        (goto _label_2)
        (else
          (set `self.TrapInvenoryIndex` _returnvalue_3))))
    (:`NewEnumerator2`
      (if (== _returnvalue -1)
        (set `self.TrapList` "NewEnumerator0")
        (goto _label_2)
        (else
          (set `self.TrapInvenoryIndex` _returnvalue)))))
  (`KismetSystemLibrary.PrintString` (`KismetStringLibrary.Conv_IntToString` (`self.TrapInvenoryIndex`))))