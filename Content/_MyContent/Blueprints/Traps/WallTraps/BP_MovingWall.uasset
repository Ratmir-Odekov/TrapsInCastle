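; Moving wall trap that, when activated, slides out and knocks back actors it hits.
; ActivateTrap spawns the mesh and collision, drives the wall's relative X with a timeline, then despawns it after a delay and starts the cooldown.
; Collision box overlaps apply a fixed X-axis impulse through the trap status effect component, with a debug print.
; Spawn and despawn extend parent logic by toggling mesh and collision.
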(event `self.ReceiveBeginPlay`
  (`parent.ReceiveBeginPlay`)
  (`self.DespawnTrap`))

(event `self.ActivateTrap`
  (bind _wall (`self.Wall`))
  (bind (_relativelocation_x _relativelocation_y _relativelocation_z) (`KismetMathLibrary.BreakVector` (`SceneComponent.RelativeLocation` _wall)))
  (bind _newparam (`self.SetTrapActive`))
  (if _newparam
    (`self.SpawnTrap`)
    ; Need to edit this part. Wall needs to move, not grow
    (bind (_direction _newtrack_0) (`Timeline|MovingWallActivation` :!via `PlayFromStart`)
      (:`Update`
        (`SceneComponent.K2_SetRelativeLocation` _wall (`KismetMathLibrary.MakeVector` _newtrack_0 _relativelocation_y _relativelocation_z) false false))
      (:`Finished`
        (`KismetSystemLibrary.Delay` (`self.DespawnTime`))
        (`self.DespawnTrap`)
        (`self.TrapCooldown`)))))

(event `self.CollisionBox.OnComponentBeginOverlap`
  (params (OverlappedComponent :type "PrimitiveComponent Object Reference") (OtherActor :type "Actor Object Reference") (OtherComp :type "PrimitiveComponent Object Reference") (OtherBodyIndex :type Integer) (bFromSweep :type Boolean) (SweepResult :type "HitResult Structure (by ref)"))
  (`self.CheckHitActor` OtherActor)
  (`KismetSystemLibrary.PrintString` (`KismetSystemLibrary.GetDisplayName` OtherActor))
  (`/Game/_MyContent/Components/BPC_TrapStatusEffect.FlyingImpuls` (`self.BPC_TrapStatusEffect`) (`self.LocalHitActor`) (10000.0 0.0 0.0))
  (`KismetArrayLibrary.Array_RemoveItem` (`self.HitActors`) (`self.LocalHitActor`)))

(fn `DespawnTrap`
  (`parent.DespawnTrap`)
  (`StaticMeshComponent.SetStaticMesh` (`self.Wall`) null)
  (`PrimitiveComponent.SetCollisionEnabled` (`self.CollisionBox`) "NoCollision"))

(fn `SpawnTrap`
  (`parent.SpawnTrap`)
  (`StaticMeshComponent.SetStaticMesh` (`self.Wall`) (`self.WallStaticMesh`))
  (`PrimitiveComponent.SetCollisionEnabled` (`self.CollisionBox`) "QueryAndPhysics"))

(fn `UserConstructionScript`
  (`parent.UserConstructionScript`))