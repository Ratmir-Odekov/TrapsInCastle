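; Base trap Blueprint that provides readiness, activation and hit-tracking logic for traps, presumably extended by child traps.
; A cooldown started on BeginPlay sets TrapReady; ActivateTrap and SetTrapActive consume it or play an invalid-action sound, without restarting the cooldown here.
; CheckHitActor records actors in HitActors to flag repeat hits, while the CheckHitActors macro only branches on membership.
; SpawnTrap clears the TrapSpot mesh, and DespawnTrap restores its marker mesh and material.
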(event `self.ReceiveBeginPlay`
  (`self.TrapCooldown`))

(event `TrapCooldown`
  (`KismetSystemLibrary.Delay` (`self.Cooldown`))
  (set `self.TrapReady?` true))

(event `ActivateTrap`
  (if (`self.TrapReady?`)
    (set `self.TrapReady?` false)
    (else
      (`GameplayStatics.SpawnSound2D` "/Engine/VREditor/Sounds/UI/Invalid_Action.Invalid_Action" 1.0 1.0 0.0 null))))

(fn `CheckHitActor`
  (params (HitActor :type "Actor Object Reference"))
  (returns (`OldHitActor?` :type Boolean))
  (`/Engine/EditorBlueprintResources/StandardMacros.IsValid` HitActor
    (:`Is Valid`
      (if (`KismetArrayLibrary.Array_Contains` (`self.HitActors`) HitActor)
        (return true)
        (else
          (`KismetArrayLibrary.Array_AddUnique` (`self.HitActors`) HitActor)
          (return false))))))

(fn `DespawnTrap`
  (`StaticMeshComponent.SetStaticMesh` (`self.TrapSpot`) (`self.DespawnSMStar`))
  (`PrimitiveComponent.SetMaterial` (`self.TrapSpot`) 0 (`self.TrapSpotMaterial`)))

(fn `SetTrapActive`
  (returns (NewParam :type Boolean))
  (bind _trapready_ (`self.TrapReady?`))
  (bind _returnvalue (`KismetStringLibrary.Conv_BoolToString` _trapready_))
  (if _trapready_
    (`KismetSystemLibrary.PrintString` _returnvalue)
    (set `self.TrapReady?` false)
    (return true)
    (else
      (`KismetSystemLibrary.PrintString` _returnvalue)
      (`GameplayStatics.SpawnSound2D` "/Engine/VREditor/Sounds/UI/Invalid_Action.Invalid_Action" 1.0 1.0 0.0 null)
      (return false))))

(fn `SpawnTrap`
  (`StaticMeshComponent.SetStaticMesh` (`self.TrapSpot`) null))

(fn `UserConstructionScript`)