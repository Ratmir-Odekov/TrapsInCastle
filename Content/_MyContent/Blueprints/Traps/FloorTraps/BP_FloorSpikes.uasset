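; Floor spike trap, a child of a parent trap class, that damages and launches actors that touch it.
; It stays hidden without meshes or collision until activated, then a timeline moves the spikes, and after a delay it despawns and starts its cooldown.
; Overlaps pass a hit-actor check before the damage and status effect components apply a hit and impulse, with brief tracking to limit repeats.
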(event `self.ReceiveBeginPlay`
  (`parent.ReceiveBeginPlay`)
  (`self.DespawnTrap`))

(event `self.ActivateTrap`
  (bind _newparam (`self.SetTrapActive`))
  (if _newparam
    (`self.SpawnTrap`)
    (`PrimitiveComponent.SetCollisionEnabled` (`self.CollisionBox`) "QueryAndProbe")
    (bind (_direction _newtrack_0) (`Timeline|SpikesUpAndDown` :!via `PlayFromStart`)
      (:`Update`
        (`SceneComponent.K2_SetRelativeLocation` (`self.Spikes`) (`KismetMathLibrary.MakeVector` 0.0 0.0 _newtrack_0) false false))
      (:`Finished`
        (`KismetSystemLibrary.Delay` (`self.DespawnTime`))
        (`self.DespawnTrap`)
        (`self.TrapCooldown`)))))

(event `self.CollisionBox.OnComponentBeginOverlap`
  (params (OverlappedComponent :type "PrimitiveComponent Object Reference") (OtherActor :type "Actor Object Reference") (OtherComp :type "PrimitiveComponent Object Reference") (OtherBodyIndex :type Integer) (bFromSweep :type Boolean) (SweepResult :type "HitResult Structure (by ref)"))
  (bind _oldhitactor_ (`self.CheckHitActor` OtherActor))
  (if (not _oldhitactor_)
    (`/Game/_MyContent/Components/BPC_DamageDeal.SingleTimeDamage` (`self.BPC_DamageDeal`) (`self.LocalHitActor`))
    (`/Game/_MyContent/Components/BPC_TrapStatusEffect.FlyingImpuls` (`self.BPC_TrapStatusEffect`) (`self.LocalHitActor`) (* (1.0 10.0 200.0) (`/Game/_MyContent/Components/BPC_TrapStatusEffect.ImpulsePower` (`self.BPC_TrapStatusEffect`))))
    (`KismetSystemLibrary.Delay` 0.5)
    (`KismetArrayLibrary.Array_RemoveItem` (`self.HitActors`) (`self.LocalHitActor`))))

(fn `DespawnTrap`
  (`parent.DespawnTrap`)
  (`StaticMeshComponent.SetStaticMesh` (`self.FloorBase`) null)
  (`StaticMeshComponent.SetStaticMesh` (`self.Spikes`) null)
  (`PrimitiveComponent.SetCollisionEnabled` (`self.CollisionBox`) "NoCollision"))

(fn `SpawnTrap`
  (`parent.SpawnTrap`)
  (`StaticMeshComponent.SetStaticMesh` (`self.FloorBase`) (`self.FloorBaseSM`))
  (`StaticMeshComponent.SetStaticMesh` (`self.Spikes`) (`self.SpikesSM`))
  (`PrimitiveComponent.SetCollisionEnabled` (`self.CollisionBox`) "QueryAndPhysics"))

(fn `UserConstructionScript`
  (`parent.UserConstructionScript`))