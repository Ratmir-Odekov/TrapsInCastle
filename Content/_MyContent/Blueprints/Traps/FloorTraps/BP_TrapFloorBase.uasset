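; BP_TrapFloorBase is a floor trap base Blueprint that extends a parent trap class.
; On BeginPlay it sends a reference to itself to player pawn 0 through FloorTrapRefMessage.
; Interface events let callers trigger it through ActivateTrap or remove it by destroying the actor.
; The construction script and DespawnTrap only call their parent versions.
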(event `self.ReceiveBeginPlay`
  (`parent.ReceiveBeginPlay`)
  (message `/Game/_MyContent/Interfaces/BPI_TrapDataShare.FloorTrapRef` (`GameplayStatics.GetPlayerPawn` 0) self))

(event `/Game/_MyContent/Interfaces/BPI_FloorTrapInterface.FloorTrapActivation`
  (`self.ActivateTrap`))

(event `/Game/_MyContent/Interfaces/BPI_FloorTrapInterface.RemoveFloorTrap`
  (`self.K2_DestroyActor`))

(fn `DespawnTrap`
  (`parent.DespawnTrap`))

(fn `UserConstructionScript`
  (`parent.UserConstructionScript`))