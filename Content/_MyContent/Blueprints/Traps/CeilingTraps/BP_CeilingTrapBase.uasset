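; Base Blueprint for ceiling traps, extending a parent trap class.
; On BeginPlay it passes a reference to itself to the player pawn through a CeilingTrapRef message.
; The CeilingTrapActivation event triggers ActivateTrap.
; Its DespawnTrap override runs the parent logic, then sets the TrapSpot material to the ceiling trap star.
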(event `self.ReceiveBeginPlay`
  (`parent.ReceiveBeginPlay`)
  (message `/Game/_MyContent/Interfaces/BPI_TrapDataShare.CeilingTrapRef` (`GameplayStatics.GetPlayerPawn` 0) self))

(event `/Game/_MyContent/Interfaces/BPI_CeilingTrapInterface.CeilingTrapActivation`
  (`self.ActivateTrap`))

(fn `DespawnTrap`
  (`parent.DespawnTrap`)
  (`PrimitiveComponent.SetMaterial` (`self.TrapSpot`) 0 "/Game/Fab/Star_effect_low_poly_137KB/star_effect_low_poly_transparency/Materials/MI_CeilingTrapStar.MI_CeilingTrapStar"))

(fn `UserConstructionScript`
  (`parent.UserConstructionScript`))