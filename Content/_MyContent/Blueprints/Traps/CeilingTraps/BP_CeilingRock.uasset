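; Ceiling rock trap, a child trap Blueprint that damages and knocks back actors hit by its rock.
; Activation shows the rock mesh and enables its hit sphere, then despawns after a delay, hiding the rock and teleporting it to its start position.
; Sphere overlaps, filtered by a hit-actor check, deal single-time damage and a velocity-scaled impulse through damage and status-effect components.
; Cooldown is called both on spawn and after despawn.
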(event `self.ReceiveBeginPlay`
  (`parent.ReceiveBeginPlay`)
  (set `self.InitialRockPosition` (`SceneComponent.K2_GetComponentLocation` (`self.Rock`)))
  (`self.DespawnTrap`))

(event `self.ActivateTrap`
  (bind _newparam (`self.SetTrapActive`))
  (if _newparam
    (`self.SpawnTrap`)
    (`KismetSystemLibrary.Delay` (`self.DespawnTime`))
    (`self.DespawnTrap`)
    ; Only after rock disappears
    (`self.TrapCooldown`)))

(event `self.Sphere.OnComponentBeginOverlap`
  (params (OverlappedComponent :type "PrimitiveComponent Object Reference") (OtherActor :type "Actor Object Reference") (OtherComp :type "PrimitiveComponent Object Reference") (OtherBodyIndex :type Integer) (bFromSweep :type Boolean) (SweepResult :type "HitResult Structure (by ref)"))
  (bind _oldhitactor_ (`self.CheckHitActor` OtherActor))
  (if (not _oldhitactor_)
    (`/Game/_MyContent/Components/BPC_DamageDeal.SingleTimeDamage` (`self.BPC_DamageDeal`) (`self.LocalHitActor`))
    (`/Game/_MyContent/Components/BPC_TrapStatusEffect.FlyingImpuls` (`self.BPC_TrapStatusEffect`) (`self.LocalHitActor`) (* (`SceneComponent.GetComponentVelocity` (`self.Rock`)) (`/Game/_MyContent/Components/BPC_TrapStatusEffect.ImpulsePower` (`self.BPC_TrapStatusEffect`))))
    (`KismetArrayLibrary.Array_RemoveItem` (`self.HitActors`) (`self.LocalHitActor`))
    (`KismetSystemLibrary.PrintString` "HitActor removed")))

(fn `DespawnTrap`
  (`parent.DespawnTrap`)
  (`StaticMeshComponent.SetStaticMesh` (`self.Rock`) null)
  (`SceneComponent.K2_SetWorldLocation` (`self.Rock`) (`self.InitialRockPosition`) false true)
  (`PrimitiveComponent.SetCollisionEnabled` (`self.Sphere`) "NoCollision"))

(fn `SpawnTrap`
  (`parent.SpawnTrap`)
  (`StaticMeshComponent.SetStaticMesh` (`self.TrapSpot`) null)
  (`StaticMeshComponent.SetStaticMesh` (`self.Rock`) (`self.RockMesh`))
  (`PrimitiveComponent.SetCollisionEnabled` (`self.Sphere`) "QueryAndPhysics")
  (`self.TrapCooldown`))

(fn `UserConstructionScript`
  (`parent.UserConstructionScript`))