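; Base player character Blueprint that lets the player place, activate and remove one floor, wall and ceiling trap each.
; In trap mode, Tick traces from the camera, snaps the hit to a grid, box-checks the cell and colors a preview mesh green or red.
; Trap inputs spawn inventory traps in trap mode, otherwise messaging stored trap references, which arrive through interface events.
; BeginPlay shares the player and health with the controller.
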(event `EnhancedInput|/Game/Input/Actions/IA_RemoveFloorTrap`
  (params (ActionValue :type Boolean) (ElapsedSeconds :type "Float (double-precision)") (TriggeredSeconds :type "Float (double-precision)") (InputAction :type "InputAction Object Reference" :default "/Game/Input/Actions/IA_RemoveFloorTrap.IA_RemoveFloorTrap"))
  (bind _floor_trap_ref (`self.Floor Trap Ref`))
  (:`Started`
    (`/Engine/EditorBlueprintResources/StandardMacros.IsValid` _floor_trap_ref
      (:`Is Valid`
        (message `/Game/_MyContent/Interfaces/BPI_FloorTrapInterface.RemoveFloorTrap` _floor_trap_ref)
        ; CharBlueprint must have an "inventory" of traps where player selects the trap to place
        (set `self.Floor Trap Ref` null)))))

(event `EnhancedInput|/Game/Input/Actions/IA_RemoveWallTrap`
  (params (ActionValue :type Boolean) (ElapsedSeconds :type "Float (double-precision)") (TriggeredSeconds :type "Float (double-precision)") (InputAction :type "InputAction Object Reference" :default "/Game/Input/Actions/IA_RemoveWallTrap.IA_RemoveWallTrap"))
  (bind _wall_trap_ref (`self.Wall Trap Ref`))
  (:`Started`
    (`/Engine/EditorBlueprintResources/StandardMacros.IsValid` _wall_trap_ref
      (:`Is Valid`
        (message `/Game/_MyContent/Interfaces/BPI_WallTrapInterface.RemoveWallTrap` _wall_trap_ref)
        ; CharBlueprint must have an "inventory" of traps where player selects the trap to place
        (set `self.Wall Trap Ref` null)))))

(event `EnhancedInput|/Game/Input/Actions/IA_RemoveCeilingTrap`
  (params (ActionValue :type Boolean) (ElapsedSeconds :type "Float (double-precision)") (TriggeredSeconds :type "Float (double-precision)") (InputAction :type "InputAction Object Reference" :default "/Game/Input/Actions/IA_RemoveCeilingTrap.IA_RemoveCeilingTrap"))
  (bind _ceiling_trap_ref (`self.Ceiling Trap Ref`))
  (:`Started`
    (`/Engine/EditorBlueprintResources/StandardMacros.IsValid` _ceiling_trap_ref
      (:`Is Valid`
        (message `/Game/_MyContent/Interfaces/BPI_CeilingTrapInterface.RemoveCeilingTrap` _ceiling_trap_ref)
        ; CharBlueprint must have an "inventory" of traps where player selects the trap to place
        (set `self.Ceiling Trap Ref` null)))))

(event `EnhancedInput|/Game/Input/Actions/IA_TrapMode`
  (params (ActionValue :type Boolean) (ElapsedSeconds :type "Float (double-precision)") (TriggeredSeconds :type "Float (double-precision)") (InputAction :type "InputAction Object Reference" :default "/Game/Input/Actions/IA_TrapMode.IA_TrapMode"))
  (:`Started`
    (message `/Game/_MyContent/Interfaces/BPI_HUD.TrapModeSingToController` (`GameplayStatics.GetPlayerController` 0))
    (`/Engine/EditorBlueprintResources/StandardMacros.FlipFlop`
      (:`A`
        (set `self.TrapMode?` true)
        (`StaticMeshComponent.SetStaticMesh` (`self.TrapLocationPreview`) (`self.TrapLocationPreviewMesh`)))
      (:`B`
        (set `self.TrapMode?` false)
        (`StaticMeshComponent.SetStaticMesh` (`self.TrapLocationPreview`) null)))))

(event `EnhancedInput|/Game/Input/Actions/IA_FloorTrap`
  (params (ActionValue :type Boolean) (ElapsedSeconds :type "Float (double-precision)") (TriggeredSeconds :type "Float (double-precision)") (InputAction :type "InputAction Object Reference" :default "/Game/Input/Actions/IA_FloorTrap.IA_FloorTrap"))
  (:`Started`
    (if (`self.TrapMode?`)
      (if (`self.IsCellAvailable?`)
        (`/Engine/EditorBlueprintResources/StandardMacros.IsValid` (`self.Floor Trap Ref`)
          (:`Is Valid`
            (`GameplayStatics.SpawnSound2D` "/Engine/VREditor/Sounds/UI/Invalid_Action.Invalid_Action" 1.0 1.0 0.0 null))
          (:`Is Not Valid`
            (`|SpawnActorFromClass` (`.TrapClass_6_B6EEF7F042E756A555B1F6B329327BE7` (break `/Game/_MyContent/DataTables/Struct_TrapAsset` (`/Game/_MyContent/Blueprints/DataAsset/BP_TrapBlueprint.TrapInfo` (`|GetArrayItem` (`self.TrapInventoryFloor`))))) (`KismetMathLibrary.MakeTransform` (`self.TrapModeLocation`)) "Undefined" "MultiplyWithRoot" null null)))
        (else
          (`GameplayStatics.SpawnSound2D` "/Engine/VREditor/Sounds/UI/Invalid_Action.Invalid_Action" 1.0 1.0 0.0 null)))
      (else
        (message `/Game/_MyContent/Interfaces/BPI_FloorTrapInterface.FloorTrapActivation` (`self.Floor Trap Ref`))))))

(event `EnhancedInput|/Game/Input/Actions/IA_WallTrap`
  (params (ActionValue :type Boolean) (ElapsedSeconds :type "Float (double-precision)") (TriggeredSeconds :type "Float (double-precision)") (InputAction :type "InputAction Object Reference" :default "/Game/Input/Actions/IA_WallTrap.IA_WallTrap"))
  (:`Started`
    (if (`self.TrapMode?`)
      (if (`self.IsCellAvailable?`)
        (`/Engine/EditorBlueprintResources/StandardMacros.IsValid` (`self.Wall Trap Ref`)
          (:`Is Valid`
            (`GameplayStatics.SpawnSound2D` "/Engine/VREditor/Sounds/UI/Invalid_Action.Invalid_Action" 1.0 1.0 0.0 null))
          (:`Is Not Valid`
            (`|SpawnActorFromClass` (`.TrapClass_6_B6EEF7F042E756A555B1F6B329327BE7` (break `/Game/_MyContent/DataTables/Struct_TrapAsset` (`/Game/_MyContent/Blueprints/DataAsset/BP_TrapBlueprint.TrapInfo` (`|GetArrayItem` (`self.TrapInventoryFloor`) 1)))) (`KismetMathLibrary.MakeTransform` (`self.TrapModeLocation`)) "Undefined" "MultiplyWithRoot" null null)))
        (else
          (`GameplayStatics.SpawnSound2D` "/Engine/VREditor/Sounds/UI/Invalid_Action.Invalid_Action" 1.0 1.0 0.0 null)))
      (else
        (message `/Game/_MyContent/Interfaces/BPI_WallTrapInterface.WallTrapActivation` (`self.Wall Trap Ref`))))))

(event `EnhancedInput|/Game/Input/Actions/IA_CeilingTrap`
  (params (ActionValue :type Boolean) (ElapsedSeconds :type "Float (double-precision)") (TriggeredSeconds :type "Float (double-precision)") (InputAction :type "InputAction Object Reference" :default "/Game/Input/Actions/IA_CeilingTrap.IA_CeilingTrap"))
  (:`Started`
    (if (`self.TrapMode?`)
      (if (`self.IsCellAvailable?`)
        (`/Engine/EditorBlueprintResources/StandardMacros.IsValid` (`self.Ceiling Trap Ref`)
          (:`Is Valid`
            (`GameplayStatics.SpawnSound2D` "/Engine/VREditor/Sounds/UI/Invalid_Action.Invalid_Action" 1.0 1.0 0.0 null))
          (:`Is Not Valid`
            (`|SpawnActorFromClass` (`.TrapClass_6_B6EEF7F042E756A555B1F6B329327BE7` (break `/Game/_MyContent/DataTables/Struct_TrapAsset` (`/Game/_MyContent/Blueprints/DataAsset/BP_TrapBlueprint.TrapInfo` (`|GetArrayItem` (`self.TrapInventoryFloor`) 2)))) (`KismetMathLibrary.MakeTransform` (`self.TrapModeLocation`)) "Undefined" "MultiplyWithRoot" null null)))
        (else
          (`GameplayStatics.SpawnSound2D` "/Engine/VREditor/Sounds/UI/Invalid_Action.Invalid_Action" 1.0 1.0 0.0 null)))
      (else
        (message `/Game/_MyContent/Interfaces/BPI_CeilingTrapInterface.CeilingTrapActivation` (`self.Ceiling Trap Ref`))))))

(event `self.ReceiveBeginPlay`
  (`parent.ReceiveBeginPlay`)
  (message `/Game/_MyContent/Interfaces/BPI_HUD.SharePlayerRef` (`GameplayStatics.GetPlayerController` 0) self)
  (message `/Game/_MyContent/Interfaces/BPI_HUD.UpdatePlayerHealthInController` (`GameplayStatics.GetPlayerController` 0) (/ (`/Game/_MyContent/Components/BPC_Health.CurrentHealth` (`self.BPC_Health`)) 100.0)))

(event `self.ReceiveTick`
  (params (DeltaSeconds :type "Float (single-precision)"))
  (bind _returnvalue (`SceneComponent.K2_GetComponentLocation` (`self.FollowCamera`)))
  (if (`self.TrapMode?`)
    (bind (_outhit _returnvalue_2) (`KismetSystemLibrary.LineTraceSingle` :`Start` _returnvalue :`End` (+ _returnvalue (* (`SceneComponent.GetForwardVector` (`self.FollowCamera`)) 1000.0)) :`TraceChannel` "TraceTypeQuery1" :`DrawDebugType` "ForOneFrame"))
    (if _returnvalue_2
      (bind _snappedlocation (`/Game/_MyContent/BPFunctionLibrary/BPFL_GridTrapSystem.SnapVectorToGrid` (`.ImpactPoint` (`GameplayStatics.BreakHitResult` _outhit)) 200.0 (`.Normal` (`GameplayStatics.BreakHitResult` _outhit))))
      (bind _output_get (set `self.TrapModeLocation` _snappedlocation))
      (bind _isavailable (`self.IsCellAvailable` _output_get (`.ImpactNormal` (`GameplayStatics.BreakHitResult` _outhit))))
      (bind _output_get_2 (set `self.IsCellAvailable?` _isavailable))
      (if _output_get_2
        (`PrimitiveComponent.SetMaterial` (`self.TrapLocationPreview`) 0 (`self.TrapLocationPrevewMatGreen`))
        (else
          (`PrimitiveComponent.SetMaterial` (`self.TrapLocationPreview`) 0 (`self.TrapLocationPrevewMatRed`))))
      (`SceneComponent.K2_SetWorldLocationAndRotation` (`self.TrapLocationPreview`) (`self.TrapModeLocation`) (`KismetMathLibrary.MakeRotFromZ` (`.Normal` (`GameplayStatics.BreakHitResult` _outhit))) false true))))

(event `/Game/_MyContent/Interfaces/BPI_TrapDataShare.WallTrapRef`
  (params (WallTrapRef :type "/Game/_MyContent/Blueprints/Traps/WallTraps/BP_WallTrapBase Object Reference"))
  (set `self.Wall Trap Ref` WallTrapRef))

(event `/Game/_MyContent/Interfaces/BPI_TrapDataShare.CeilingTrapRef`
  (params (CeilingTrapRef :type "/Game/_MyContent/Blueprints/Traps/CeilingTraps/BP_CeilingTrapBase Object Reference"))
  (set `self.Ceiling Trap Ref` CeilingTrapRef))

(event `/Game/_MyContent/Interfaces/BPI_TrapDataShare.FloorTrapRef`
  (params (FloorTrapRef :type "/Game/_MyContent/Blueprints/Traps/FloorTraps/BP_TrapFloorBase Object Reference"))
  (set `self.Floor Trap Ref` FloorTrapRef))

(fn `IsCellAvailable`
  (params (CheckLocation :type "Vector Structure") (Normal :type "Vector Structure"))
  (returns (IsAvailable :type Boolean))
  (bind _returnvalue (+ CheckLocation (* Normal 100.0)))
  (bind (_outhit _returnvalue_2) (`KismetSystemLibrary.BoxTraceSingle` _returnvalue (+ _returnvalue (0.0 0.0 1.0)) (70.0 70.0 70.0) (struct) "TraceTypeQuery1"))
  (return (not _returnvalue_2)))

(fn `UserConstructionScript`
  (`parent.UserConstructionScript`))